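; Trigger actor that starts a game encounter when a BP_CDPaperCharacter overlaps its collision component.
; On overlap it adds a new WBP_GameScore widget to the viewport and plays the SW_Game sound.
; It also spawns a BP_CDAICharacter after SpawnDelay, offset from the trigger's location by SpawnDelta.
; The graph has no one-shot guard, so each qualifying overlap creates another widget and sound.
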(event OnComponentBeginOverlap(CollisionComponent)
  (params (OverlappedComponent :type Primitive%20Component%20Object%20Reference) (OtherActor :type Actor%20Object%20Reference) (OtherComp :type Primitive%20Component%20Object%20Reference) (OtherBodyIndex :type Integer) (bFromSweep :type Boolean) (SweepResult :type Hit%20Result%20Structure%20%28by%20ref%29))
  (Utilities|Casting|CastToBP_CDPaperCharacter OtherActor)
  (Utilities|FlowControl|Sequence
    (:then_0
      (bind _returnvalue (UserInterface|CreateWidget "/Game/UI/WBP_GameScore.WBP_GameScore_C"))
      (UserInterface|Viewport|AddtoViewport _returnvalue 1)
      (Audio|PlaySound2D "/Game/Audio/SW_Game.SW_Game" 1.0 1.0 0.0 0 0))
    (:then_1
      (Utilities|FlowControl|Delay (Variables|Default|GetSpawnDelay))
      (Game|SpawnActorfromClass "/Game/AI/BP_CDAICharacter.BP_CDAICharacter_C" (Math|Conversions|ToTransform(Vector) (+ (Transformation|GetActorLocation) (Variables|Default|GetSpawnDelta))) "Undefined" "MultiplyWithRoot" 0 0))))

(event EventBeginPlay)

(event Collision|EventActorBeginOverlap
  (params (OtherActor :type Actor%20Object%20Reference)))

(event EventTick
  (params (DeltaSeconds :type Float%20%28single-precision%29)))

(fn ConstructionScript)