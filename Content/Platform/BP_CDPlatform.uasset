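; Platform actor that can spawn random obstacle blocks, knocks characters off its side meshes and pulses two point lights.
; On BeginPlay, if SpawnBlocks is set, each of three targets randomly receives an actor from the BlockOption map, destroyed on EndPlay.
; Left and right mesh hits launch Characters along the negated hit normal.
; Tick ramps both lights between intensity limits, reversing through a shared IsUp flag.
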(event OnComponentHit(LeftMesh)
  (params (HitComponent :type Primitive%20Component%20Object%20Reference) (OtherActor :type Actor%20Object%20Reference) (OtherComp :type Primitive%20Component%20Object%20Reference) (NormalImpulse :type Vector :default "0, 0, 0") (Hit :type Hit%20Result%20Structure%20%28by%20ref%29))
  (bind _ascharacter (Utilities|Casting|CastToCharacter OtherActor))
  (Character|LaunchCharacter _ascharacter (* (.normal Hit) (Variables|Default|GetLaunchSpeed) -1.0) false false))

(event OnComponentHit(RightMesh)
  (params (HitComponent :type Primitive%20Component%20Object%20Reference) (OtherActor :type Actor%20Object%20Reference) (OtherComp :type Primitive%20Component%20Object%20Reference) (NormalImpulse :type Vector :default "0, 0, 0") (Hit :type Hit%20Result%20Structure%20%28by%20ref%29))
  (bind _ascharacter (Utilities|Casting|CastToCharacter OtherActor))
  (Character|LaunchCharacter _ascharacter (* (.normal Hit) (Variables|Default|GetLaunchSpeed) -1.0) false false))

(event EventBeginPlay
  (bind _blockoption (Variables|Default|GetBlockOption))
  (if (Variables|Default|GetSpawnBlocks)
    (Utilities|FlowControl|Sequence
      (:then_0
        (Utilities|Array|Add (Variables|Default|GetTargetArray) (Variables|Default|GetTarget1))
        (Utilities|Array|Add (Variables|Default|GetTargetArray) (Variables|Default|GetTarget2))
        (Utilities|Array|Add (Variables|Default|GetTargetArray) (Variables|Default|GetTarget3)))
      (:then_1
        (for _array_element (Variables|Default|GetTargetArray)
          (if (Math|Random|RandomBool)
            (bind _returnvalue (Game|SpawnActorfromClass (.Value (Utilities|Map|Find _blockoption (Math|Random|RandomIntegerinRange 0 (Utilities|Map|Length _blockoption)))) (Transformation|GetWorldTransform _array_element) "Undefined" "MultiplyWithRoot" 0 0))
            (Utilities|Array|Add (Variables|Default|GetBlockArray) _returnvalue)))))))

(event EventEndPlay
  (params (EndPlayReason :type EEndPlayReason%20Enum :default "Destroyed"))
  (for _array_element (Variables|Default|GetBlockArray)
    (if (Utilities|IsValid _array_element)
      (Actor|DestroyActor _array_element))))

(event EventTick
  (params (DeltaSeconds :type Float%20%28single-precision%29))
  (bind _pointlight1 (Variables|Default|GetPointLight1))
  (bind _flickspeed (Variables|Default|GetFlickSpeed))
  (bind _pointlight1_2 (Variables|Default|GetPointLight1))
  (bind _pointlight2 (Variables|Default|GetPointLight2))
  (bind _pointlight2_2 (Variables|Default|GetPointLight2))
  (bind _flickspeed_2 (Variables|Default|GetFlickSpeed))
  (bind _flickspeed_3 (Variables|Default|GetFlickSpeed))
  (bind _flickspeed_4 (Variables|Default|GetFlickSpeed))
  (bind _returnvalue (* DeltaSeconds _flickspeed_2 -1.0))
  (bind _returnvalue_2 (* DeltaSeconds _flickspeed))
  (bind _returnvalue_3 (* DeltaSeconds _flickspeed_3 -1.0))
  (bind _returnvalue_4 (* DeltaSeconds _flickspeed_4))
  (bind _intensity (Variables|/Script/Engine.LightComponentBase|GetIntensity _pointlight2))
  (bind _intensity_2 (Variables|/Script/Engine.LightComponentBase|GetIntensity _pointlight2_2))
  (bind _intensity_3 (Variables|/Script/Engine.LightComponentBase|GetIntensity _pointlight1))
  (bind _intensity_4 (Variables|/Script/Engine.LightComponentBase|GetIntensity _pointlight1_2))
  (bind _returnvalue_5 (+ _intensity_3 _returnvalue_4))
  (bind _returnvalue_6 (+ _intensity_4 _returnvalue_3))
  (bind _returnvalue_7 (+ _intensity _returnvalue))
  (bind _returnvalue_8 (+ _intensity_2 _returnvalue_2))
  (Utilities|FlowControl|Sequence
    (:then_0
      (if (Variables|Default|GetbIsUp)
        (if (and (> _returnvalue_5 (Variables|Default|GetMinIntecity)) (< _returnvalue_5 (Variables|Default|GetMaxIntecity)))
          (Rendering|Components|Light|SetIntensity _pointlight1 _returnvalue_5)
          (else
            (Variables|Default|SetbIsUp false)))
        (elif (and (> _returnvalue_6 (Variables|Default|GetMinIntecity)) (< _returnvalue_6 (Variables|Default|GetMaxIntecity)))
          (Rendering|Components|Light|SetIntensity _pointlight1_2 _returnvalue_6)
          (else
            (Variables|Default|SetbIsUp true)))))
    (:then_1
      (if (Variables|Default|GetbIsUp)
        (if (and (> _returnvalue_8 (Variables|Default|GetMinIntecity)) (< _returnvalue_8 (Variables|Default|GetMaxIntecity)))
          (Rendering|Components|Light|SetIntensity _pointlight2_2 _returnvalue_8)
          (else
            (Variables|Default|SetbIsUp false)))
        (elif (and (> _returnvalue_7 (Variables|Default|GetMinIntecity)) (< _returnvalue_7 (Variables|Default|GetMaxIntecity)))
          (Rendering|Components|Light|SetIntensity _pointlight2 _returnvalue_7)
          (else
            (Variables|Default|SetbIsUp true)))))))

(fn ConstructionScript)