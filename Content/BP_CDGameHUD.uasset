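; HUD Blueprint that manages the game's top-level screens, input mode and mouse cursor.
; On BeginPlay it caches BP_CDGameMode, then shows the main menu with sound in MenuLevel, or the gameplay overlay in other levels.
; Tick polls the game mode for game over and, through a DoOnce that resets when play resumes, shows either the abuse-over or game-over screen with UI-only input.
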(event EventBeginPlay
  (bind _returnvalue (Game|Player|GetOwningPlayerController))
  (bind _returnvalue_2 (Game|Player|GetOwningPlayerController))
  (Utilities|FlowControl|Sequence
    (:then_0
      (bind _asbp_cdgame_mode (Utilities|Casting|CastToBP_CDGameMode (Game|GetGameMode)))
      (Variables|Default|SetGameMode _asbp_cdgame_mode))
    (:then_1
      (bind _returnvalue_3 (Game|GetCurrentLevelName true))
      (if (Utilities|Enum|Equal(Enum) _returnvalue_3 "MenuLevel")
        (bind _returnvalue_4 (UserInterface|CreateWidget "/Game/UI/WBP_MainMenu.WBP_MainMenu_C"))
        (UserInterface|Viewport|AddtoViewport _returnvalue_4 0)
        (Input|SetInputModeUIOnly _returnvalue_2 0 "DoNotLock" false)
        (Variables|/Script/Engine.PlayerController|SetbShowMouseCursor _returnvalue_2 true)
        (Audio|PlaySound2D "/Game/Audio/SW_Menu.SW_Menu" 1.0 1.0 0.5 0 0)
        (else
          (bind _returnvalue_5 (UserInterface|CreateWidget "/Game/UI/WBP_GameOverlay.WBP_GameOverlay_C"))
          (UserInterface|Viewport|AddtoViewport _returnvalue_5 0)
          (Input|SetInputModeGameOnly _returnvalue false)
          (Variables|/Script/Engine.PlayerController|SetbShowMouseCursor _returnvalue false))))))

(event EventTick
  (params (DeltaSeconds :type Float%20%28single-precision%29))
  (bind _returnvalue (Game|Player|GetOwningPlayerController))
  (bind _returnvalue_2 (Game|Player|GetOwningPlayerController))
  (bind _result (Default|IsGameOver (Variables|Default|GetGameMode)))
  (if _result
    (Utilities|FlowControl|DoOnce false :!label _label
      (:Completed
        (bind _result_2 (Default|IsAbuseOver (Variables|Default|GetGameMode)))
        (if _result_2
          (bind _returnvalue_3 (UserInterface|CreateWidget "/Game/UI/WBP_AbuseOver.WBP_AbuseOver_C"))
          (UserInterface|Viewport|AddtoViewport _returnvalue_3 0)
          (Input|SetInputModeUIOnly _returnvalue_2 0 "DoNotLock" true)
          (Variables|/Script/Engine.PlayerController|SetbShowMouseCursor _returnvalue_2 true)
          (else
            (bind _returnvalue_4 (UserInterface|CreateWidget "/Game/UI/WBP_GameOver.WBP_GameOver_C"))
            (UserInterface|Viewport|AddtoViewport _returnvalue_4 0)
            (Input|SetInputModeUIOnly _returnvalue 0 "DoNotLock" true)
            (Variables|/Script/Engine.PlayerController|SetbShowMouseCursor _returnvalue true)))))
    (else
      (goto _label Reset))))

(fn ConstructionScript)