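; BP_CDPlatform is a platform actor that can randomly populate itself with blocks and bounces characters off its left and right meshes.
; On BeginPlay, if SpawnBlocks is set, each of three target points has a random chance to spawn a stored BP_CDBlock.
; Side-mesh hits launch characters along the negated hit normal.
; EndPlay checks each block reference, but its DestroyActor calls show no block as target.
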(event OnComponentHit(LeftMesh)
  (params (HitComponent :type Primitive%20Component%20Object%20Reference) (OtherActor :type Actor%20Object%20Reference) (OtherComp :type Primitive%20Component%20Object%20Reference) (NormalImpulse :type Vector :default "0, 0, 0") (Hit :type Hit%20Result%20Structure%20%28by%20ref%29))
  (bind _ascharacter (Utilities|Casting|CastToCharacter OtherActor))
  (Character|LaunchCharacter _ascharacter (* (.normal Hit) -5e+02) false false))

(event OnComponentHit(RightMesh)
  (params (HitComponent :type Primitive%20Component%20Object%20Reference) (OtherActor :type Actor%20Object%20Reference) (OtherComp :type Primitive%20Component%20Object%20Reference) (NormalImpulse :type Vector :default "0, 0, 0") (Hit :type Hit%20Result%20Structure%20%28by%20ref%29))
  (bind _ascharacter (Utilities|Casting|CastToCharacter OtherActor))
  (Character|LaunchCharacter _ascharacter (* (.normal Hit) -5e+02) false false))

(event EventBeginPlay
  (if (Variables|Default|GetSpawnBlocks)
    (Utilities|FlowControl|Sequence
      (:then_0
        (if (Math|Random|RandomBool)
          (bind _returnvalue (Game|SpawnActorfromClass "/Game/Platforms/BP_CDBlock.BP_CDBlock_C" (Transformation|GetWorldTransform (Variables|Default|GetTarget1)) "Undefined" "MultiplyWithRoot" 0 0))
          (Variables|Default|SetBlock1 _returnvalue)))
      (:then_1
        (if (Math|Random|RandomBool)
          (bind _returnvalue_2 (Game|SpawnActorfromClass "/Game/Platforms/BP_CDBlock.BP_CDBlock_C" (Transformation|GetWorldTransform (Variables|Default|GetTarget2)) "Undefined" "MultiplyWithRoot" 0 0))
          (Variables|Default|SetBlock2 _returnvalue_2)))
      (:then_2
        (if (Math|Random|RandomBool)
          (bind _returnvalue_3 (Game|SpawnActorfromClass "/Game/Platforms/BP_CDBlock.BP_CDBlock_C" (Transformation|GetWorldTransform (Variables|Default|GetTarget3)) "Undefined" "MultiplyWithRoot" 0 0))
          (Variables|Default|SetBlock3 _returnvalue_3))))))

(event Collision|EventActorBeginOverlap
  (params (OtherActor :type Actor%20Object%20Reference)))

(event EventTick
  (params (DeltaSeconds :type Float%20%28single-precision%29)))

(event EventEndPlay
  (params (EndPlayReason :type EEndPlayReason%20Enum :default "Destroyed"))
  (Utilities|FlowControl|Sequence
    (:then_0
      (if (Utilities|IsValid (Variables|Default|GetBlock1))
        (Actor|DestroyActor)))
    (:then_1
      (if (Utilities|IsValid (Variables|Default|GetBlock2))
        (Actor|DestroyActor)))
    (:then_2
      (if (Utilities|IsValid (Variables|Default|GetBlock3))
        (Actor|DestroyActor)))))

(fn ConstructionScript)